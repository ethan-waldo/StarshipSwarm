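; BP_FormationManager4 is a formation spawner that creates rows of enemies at its location when play begins.
; Nested loops read each RowSettings entry's class and count, stepping rows along X by EnemySpacing.
; Y is half the row's width, and the per-column spacing term is left unconnected, so each row's enemies share one spawn point.
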(event EventBeginPlay
  (for _index (range 0 (- (Utilities|Array|Length (Variables|Default|GetRowSettings)) 1)) ; Row Loop
    (bind _output_get (Variables|Default|SetCenterOffset (/ (* (Math|Conversions|ToFloat(Integer) (- (.EnemyCounter (Utilities|Struct|BreakS_EnemyRowSettings (Utilities|Array|Get(acopy) (Variables|Default|GetRowSettings) _index))) 1)) (Variables|Default|GetEnemySpacing)) 2.0)))
    (for _index_2 (range 0 (- (.EnemyCounter (Utilities|Struct|BreakS_EnemyRowSettings (Utilities|Array|Get(acopy) (Variables|Default|GetRowSettings) _index))) 1)) ; Column loop
      (Game|SpawnActorfromClass (.EnemyClass (Utilities|Struct|BreakS_EnemyRowSettings (Utilities|Array|Get(acopy) (Variables|Default|GetRowSettings) _index))) (Math|Conversions|ToTransform(Vector) (+ (Transformation|GetActorLocation) (Math|Vector|MakeVector (* _index (Variables|Default|GetEnemySpacing)) _output_get 0.0))) "Undefined" "MultiplyWithRoot" 0 0))))

(event Collision|EventActorBeginOverlap
  (params (OtherActor :type Actor%20Object%20Reference)))

(event EventTick
  (params (DeltaSeconds :type Float%20%28single-precision%29)))

(fn ConstructionScript)