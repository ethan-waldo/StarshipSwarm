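; BP_WaveManager advances the game through enemy waves and ends the run by loading the game-over map.
; Every Tick it polls for BP_Enemy actors and, when none remain, increments CurrentStage, calls SpawnWave and prints the stage.
; SpawnWave switches on the stage to spawn one of four formation manager actors at a fixed location, or to open GameOverMap once those waves are done.
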(event Custom|SpawnWave
  (bind _returnvalue (Math|Transform|MakeTransform "1090.000000,0.000000,0.000000"))
  (switch int (Variables|Default|GetCurrentStage)
    (:1
      (Game|SpawnActorfromClass "/Game/Blueprints/BP_FormationManager1.BP_FormationManager1_C" _returnvalue "Undefined" "MultiplyWithRoot" 0 5 10 1.5e+02 0 0))
    (:2
      (Game|SpawnActorfromClass "/Game/Blueprints/BP_FormationManager2.BP_FormationManager2_C" _returnvalue "Undefined" "MultiplyWithRoot" 0 5 10 1.5e+02 0 0))
    (:3
      (Game|SpawnActorfromClass "/Game/Blueprints/BP_FormationManger3.BP_FormationManger3_C" _returnvalue "Undefined" "MultiplyWithRoot" 0 5 10 1.5e+02 0 0))
    (:4
      (Game|SpawnActorfromClass "/Game/Blueprints/BP_FormationManager4.BP_FormationManager4_C" _returnvalue "Undefined" "MultiplyWithRoot" 0 5 10 1.5e+02 0 0))
    (:5
      (Game|OpenLevel(byName) "GameOverMap" :!label _label))
    (:6
      (goto _label))))

(event EventBeginPlay)

(event Collision|EventActorBeginOverlap
  (params (OtherActor :type Actor%20Object%20Reference)))

(event EventTick
  (params (DeltaSeconds :type Float%20%28single-precision%29))
  (bind _outactors (Actor|GetAllActorsOfClass "/Game/Blueprints/BP_Enemy.BP_Enemy_C"))
  (if (<= (Utilities|Array|Length _outactors) 0)
    (bind _result (Math|Integer|IncrementInt (Variables|Default|GetCurrentStage))
      (:%20%20
        (bind _output_get (Variables|Default|SetCurrentStage _result))
        (CallFunction|SpawnWave)
        (Development|PrintString (Utilities|String|ToString(Integer) _output_get))))))

(fn ConstructionScript)